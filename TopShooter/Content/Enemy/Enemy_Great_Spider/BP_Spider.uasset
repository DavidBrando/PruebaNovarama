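; Enemy spider Blueprint that links its health bar widget to itself and provides a melee-style montage attack.
; BeginPlay disables both arm colliders through ColliderSetUp, which forwards collision settings to SettingCollisionForArms, then hands itself to the EnemyHealthBar widget.
; MakeAttack plays one of two random montages, holding the Attacking flag for the returned montage duration.
; The construction script prints the controller's name as debug output.
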(event `self.ReceiveBeginPlay`
  ;[1 1 1] Setting variables
  (`parent.ReceiveBeginPlay`)
  (`self.ColliderSetUp` "NoCollision" "NoCollision")
  (bind _asenemy_health_bar (cast `/Game/UI/EnemyHealthBar` (`WidgetComponent.GetUserWidgetObject` (`self.Widget`))))
  (set `/Game/UI/EnemyHealthBar.MyPawn` self _asenemy_health_bar))

(event `Make Attack`
  ;[1 1 1] Attack system
  (set `self.attacking` true)
  (bind _returnvalue (`self.PlayAnimMontage` (select `int` (`KismetMathLibrary.RandomIntegerInRange` 0 1) :`0` "/Game/Enemy/Enemy_Great_Spider/Enemy_SpiderGreater_Animation/Atack1_Montage.Atack1_Montage" :`1` "/Game/Enemy/Enemy_Great_Spider/Enemy_SpiderGreater_Animation/Attack2_Montage.Attack2_Montage" :!type "AnimMontage Object Reference")))
  (`KismetSystemLibrary.Delay` _returnvalue)
  (set `self.attacking` false))

(event `ColliderSetUp`
  (params (Arm1 :type "ECollisionEnabled Enum" :default "NoCollision") (Arm2 :type "ECollisionEnabled Enum" :default "NoCollision"))
  ;[1 1 1] Collision system
  (`self.SettingCollisionForArms` Arm1 Arm2))

(fn `UserConstructionScript`
  (`parent.UserConstructionScript`)
  (`KismetSystemLibrary.PrintString` (`KismetSystemLibrary.GetDisplayName` (`self.GetController`))))